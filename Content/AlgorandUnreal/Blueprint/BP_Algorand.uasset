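; Actor that runs an Algorand wallet demo, bridging an AlgorandManager and the UMG wallet screens.
; BeginPlay shows the wallet widget and creates the manager with testnet Algod and Indexer endpoints.
; Manager delegates fill account creation and list widgets or print errors.
; A network settings modal edits RPC info, then refreshes the network name and sender addresses on open transaction panels, alongside UInt64 conversion and explorer-link helpers.
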(event Custom|InitWallet%20Callback
  (params (ResultType :type EResultType%20Enum%20%28by%20ref%29 :default "NONE") (Result :type Result%20Boolean%20Structure%20%28by%20ref%29))
  ;[1 1 1] Register Algorand Events to be processed on Delegate Callback
)

(event Custom|GetAllAccounts
  (params (ResultType :type EResultType%20Enum%20%28by%20ref%29 :default "NONE") (Accounts :type Result%20Accounts%20Structure%20%28by%20ref%29))
  (bind (_addresses _names) (Utilities|Struct|BreakResultAccounts Accounts))
  ;[1 1 1] Register Algorand Events to be processed on Delegate Callback
  ;[1 1 1] ALGORAND Delegate Handlers
  (if (Utilities|IsValid (Variables|Pages|Getaccountlistui))
    _
    (else
      (bind _returnvalue (UserInterface|CreateWidget "/Game/AlgorandUnreal/Blueprint/Widgets/Pages/WBP_UI_ACC_LIST.WBP_UI_ACC_LIST_C"))
      (Variables|Pages|Setaccountlistui _returnvalue)))
  (Default|RemoveObjectsonList (Variables|Pages|Getaccountlistui) (Variables|/Game/AlgorandUnreal/Blueprint/Widgets/Pages/WBP_UI_ACC_LIST.WBP_UI_ACC_LIST_C|GetAccountListView (Variables|Pages|Getaccountlistui)))
  (for _index (range 0 (- (Utilities|Array|Length _names) 1))
    (Default|AddObjecttoList (Variables|Pages|Getaccountlistui) (Utilities|Struct|MakeAccStructure (Utilities|Array|Get(acopy) _names _index) (Utilities|Array|Get(acopy) _addresses _index)) (Variables|/Game/AlgorandUnreal/Blueprint/Widgets/Pages/WBP_UI_ACC_LIST.WBP_UI_ACC_LIST_C|GetAccountListView (Variables|Pages|Getaccountlistui)))
    (UserInterface|Viewport|AddtoViewport (Variables|Pages|Getaccountlistui) 0)))

(event Custom|Error%20Callback
  (params (error :type Error%20Structure%20%28by%20ref%29))
  ;[1 1 1] Error Handler
  (Development|PrintString (Utilities|Struct|BreakError error) true true "(R=0.000000,G=0.660000,B=1.000000,A=1.000000)" 5.0))

(event Custom|CustomEvent
  (params (error :type Error%20Structure%20%28by%20ref%29))
  ;[1 1 1] Bind Error Callback
  (CallFunction|ErrorCallback error))

(event Custom|GenRandomAcc%20Callback
  (params (ResultType :type EResultType%20Enum%20%28by%20ref%29 :default "NONE") (GeneratedAccount :type Result%20Account%20Structure%20%28by%20ref%29))
  (bind (_address _name _mnemonicphrase) (Utilities|Struct|BreakResultAccount GeneratedAccount))
  ;[1 1 1] Register Algorand Events to be processed on Delegate Callback
  ;[1 1 1] ALGORAND Delegate Handlers
  (if (Utilities|IsValid (Variables|Pages|Getaccountnewui))
    _
    (else
      (bind _returnvalue (UserInterface|CreateWidget "/Game/AlgorandUnreal/Blueprint/Widgets/Pages/WBP_UI_ACC_Create.WBP_UI_ACC_Create_C"))
      (Variables|Pages|Setaccountnewui _returnvalue)))
  (Default|ConvertETBoxestoArray (Variables|Pages|Getaccountnewui))
  (Default|FIllMnemonicsinETBoxes (Variables|Pages|Getaccountnewui) _address _mnemonicphrase)
  (UserInterface|Viewport|AddtoViewport (Variables|Pages|Getaccountnewui) 0)
  (Variables|/Game/AlgorandUnreal/Blueprint/Widgets/Pages/WBP_UI_ACC_Create.WBP_UI_ACC_Create_C|SetNextAction (Variables|Pages|Getaccountnewui) (Variables|Default|GetNextAction))
  (switch string (Variables|Default|GetNextAction)
    (:NewAccount
      (Widget|RemovefromParent (Variables|Pages|Getaccountlistui)))))

(event Custom|RPC%20Updates
  (bind _getbalanceui (Variables|Pages|Getgetbalanceui))
  (bind _payui (Variables|Pages|Getpayui))
  (bind _acfgui (Variables|Pages|Getacfgui))
  (bind _axferui (Variables|Pages|Getaxferui))
  (bind _nftdetailsui (Variables|Pages|Getnftdetailsui))
  ;[1 1 1] Set Net Name On Page UI
  (bind _returnvalue (Class|AlgorandUnrealManager|GetAlgodRpcNet (Variables|Default|GetAlgorandManager)))
  (Rendering|Components|TextRender|SetText (Variables|/Game/AlgorandUnreal/Blueprint/Widgets/Pages/WBP_UI_Pages.WBP_UI_Pages_C|GetET_NetName (Variables|Pages|Getpagesui)) (Utilities|Text|ToText(String) _returnvalue))
  (Utilities|FlowControl|Sequence
    (:then_0
      ;[1 1 1] Set Address to Get Balance UI
      (if (Utilities|IsValid _getbalanceui)
        (Rendering|Components|TextRender|SetText (Variables|/Game/AlgorandUnreal/Blueprint/Widgets/Pages/WBP_UI_GET_Balance.WBP_UI_GET_Balance_C|GetEditableText_WalletAddress _getbalanceui) (Utilities|Text|ToText(String) (Variables|Account|GetMainAccountAddress)))))
    (:then_1
      ;[1 1 1] Set Address to Pay TX UI
      (if (Utilities|IsValid _payui)
        (Rendering|Components|TextRender|SetText (Variables|/Game/AlgorandUnreal/Blueprint/Widgets/Pages/WBP_UI_TX_Pay.WBP_UI_TX_Pay_C|GetEditableText_SenderAddress _payui) (Utilities|Text|ToText(String) (Variables|Account|GetMainAccountAddress)))))
    (:then_2
      (Utilities|FlowControl|Sequence
        (:then_0
          ;[1 1 1] Set Address to Acfg TX UI
          (if (Utilities|IsValid _acfgui)
            (Rendering|Components|TextRender|SetText (Variables|/Game/AlgorandUnreal/Blueprint/Widgets/Pages/WBP_UI_TX_Acfg.WBP_UI_TX_Acfg_C|GetEditableText_Creator _acfgui) (Utilities|Text|ToText(String) (Variables|Account|GetMainAccountAddress)))))
        (:then_1
          ;[1 1 1] Set Address to Axfer TX UI
          (if (Utilities|IsValid _axferui)
            (Rendering|Components|TextRender|SetText (Variables|/Game/AlgorandUnreal/Blueprint/Widgets/Pages/WBP_UI_TX_Axfer.WBP_UI_TX_Axfer_C|GetEditableText_AssetSenderAddress _axferui) (Utilities|Text|ToText(String) (Variables|Account|GetMainAccountAddress)))))
        (:then_2
          ;[1 1 1] Set Address to Arc Fetch UI
          (if (Utilities|IsValid _nftdetailsui)
            (Rendering|Components|TextRender|SetText (Variables|/Game/AlgorandUnreal/Blueprint/Widgets/Pages/WBP_UI_ARC_Fetch.WBP_UI_ARC_Fetch_C|GetEditableText_WalletAddress _nftdetailsui) (Utilities|Text|ToText(String) (Variables|Account|GetMainAccountAddress)))))))))

(event Custom|Event%20Open%20NetSettings%20UI
  ;[1 1 1] After Wallet Action, on Main Page, you can update NetSettings
  (bind _returnvalue (UserInterface|CreateWidget "/Game/AlgorandUnreal/Blueprint/Widgets/Components/Modals/WBP_MODAL_Net_Setting.WBP_MODAL_Net_Setting_C"))
  (bind _output_get (Variables|Pages|Setnetsettingsui _returnvalue))
  (EventDispatchers|BindEventtoOnClicked (Variables|/Game/AlgorandUnreal/Blueprint/Widgets/Components/Modals/WBP_MODAL_Net_Setting.WBP_MODAL_Net_Setting_C|GetButton_Net_Save (Variables|Pages|Getnetsettingsui)) (delegate Custom|Event%20Save%20Net%20Settings))
  (EventDispatchers|BindEventtoOnClicked (Variables|/Game/AlgorandUnreal/Blueprint/Widgets/Components/Modals/WBP_MODAL_Net_Setting.WBP_MODAL_Net_Setting_C|GetButton_Net_Close (Variables|Pages|Getnetsettingsui)) (delegate Custom|Event%20Close%20Net%20UI))
  (UserInterface|Viewport|AddtoViewport _output_get 0)
  (CallFunction|InitNetSettings))

(event Custom|Event%20Save%20Net%20Settings
  ;[1 1 1] After Wallet Action, on Main Page, you can update NetSettings
  (CallFunction|SaveNetSettings))

(event Custom|Event%20Close%20Net%20UI
  ;[1 1 1] After Wallet Action, on Main Page, you can update NetSettings
  (CallFunction|CloseNetSettingsUI))

(event Custom|InitializeAlgorandManger
  ;[1 1 1] Create AlgorandManager & Add Sequeunces to be run
  (if (not (Utilities|IsValid (Variables|Default|GetAlgorandManager)))
    (bind _returnvalue (Class|AlgorandUnrealManager|CreateInstancewithParams "https://testnet-api.algonode.cloud" (Class|AlgorandBPFunctionLibrary|ToUInt64(FString) (Variables|RPC|GetAlgodPort) (Class|KismetSystemLibrary|MakeLiteralBool true)) "" "https://testnet-idx.algonode.network" (Class|AlgorandBPFunctionLibrary|ToUInt64(FString) (Variables|RPC|GetIndexerPort) (Class|KismetSystemLibrary|MakeLiteralBool true)) "" (Variables|Default|GetDefaultSceneRoot)))
    (bind _output_get (Variables|Default|SetAlgorandManager _returnvalue))
    (Utilities|FlowControl|Sequence
      (:then_0
        (Utilities|FlowControl|Sequence
          (:then_0
            ;[1 1 1] Register Algorand Events to be processed on Delegate Callback
            (EventDispatchers|BindEventtoInitWalletCallback (Variables|Default|GetAlgorandManager) (delegate Custom|InitWallet%20Callback))
            (Class|AlgorandUnrealManager|InitWallet (Variables|Default|GetAlgorandManager)))
          (:then_1
            (EventDispatchers|BindEventtoGenerateRandomAccountCallback (Variables|Default|GetAlgorandManager) (delegate Custom|GenRandomAcc%20Callback)))
          (:then_2
            (EventDispatchers|BindEventtoGetAllAccountsCallback (Variables|Default|GetAlgorandManager) (delegate Custom|GetAllAccounts)))))
      (:then_1
        ;[1 1 1] Bind Error Callback
        (EventDispatchers|BindEventtoErrorDelegateCallback _output_get (delegate Custom|CustomEvent))))))

(event Custom|Save%20Net%20Settings
  (bind _netsettingsui (Variables|Pages|Getnetsettingsui))
  (bind _netsettingsui_2 (Variables|Pages|Getnetsettingsui))
  ;[1 1 1] Net Settings UI Control
  (Class|AlgorandUnrealManager|SetAlgodRpcInfo (Variables|Default|GetAlgorandManager) (Utilities|String|ToString(Text) (Class|EditableText|GetText (Variables|/Game/AlgorandUnreal/Blueprint/Widgets/Components/Modals/WBP_MODAL_Net_Setting.WBP_MODAL_Net_Setting_C|GetEditableText_Algod_RPC _netsettingsui))) (Class|AlgorandBPFunctionLibrary|ToUInt64(FString) (Utilities|String|ToString(Text) (Class|EditableText|GetText (Variables|/Game/AlgorandUnreal/Blueprint/Widgets/Components/Modals/WBP_MODAL_Net_Setting.WBP_MODAL_Net_Setting_C|GetEditableText_Algod_Port _netsettingsui))) (Class|KismetSystemLibrary|MakeLiteralBool true)) (Utilities|String|ToString(Text) (Class|EditableText|GetText (Variables|/Game/AlgorandUnreal/Blueprint/Widgets/Components/Modals/WBP_MODAL_Net_Setting.WBP_MODAL_Net_Setting_C|GetEditableText_Algod_Token _netsettingsui))))
  (Class|AlgorandUnrealManager|SetIndexerRpcInfo (Variables|Default|GetAlgorandManager) (Utilities|String|ToString(Text) (Class|EditableText|GetText (Variables|/Game/AlgorandUnreal/Blueprint/Widgets/Components/Modals/WBP_MODAL_Net_Setting.WBP_MODAL_Net_Setting_C|GetEditableText_Indexer_RPC _netsettingsui_2))) (Class|AlgorandBPFunctionLibrary|ToUInt64(FString) (Utilities|String|ToString(Text) (Class|EditableText|GetText (Variables|/Game/AlgorandUnreal/Blueprint/Widgets/Components/Modals/WBP_MODAL_Net_Setting.WBP_MODAL_Net_Setting_C|GetEditableText_Indexer_Port _netsettingsui_2))) (Class|KismetSystemLibrary|MakeLiteralBool true)) (Utilities|String|ToString(Text) (Class|EditableText|GetText (Variables|/Game/AlgorandUnreal/Blueprint/Widgets/Components/Modals/WBP_MODAL_Net_Setting.WBP_MODAL_Net_Setting_C|GetEditableText_Indexer_Token _netsettingsui_2))))
  (Widget|RemovefromParent (Variables|Pages|Getnetsettingsui))
  (CallFunction|RPCUpdates))

(event Custom|Close%20Net%20Settings%20UI
  ;[1 1 1] Net Settings UI Control
  (Widget|RemovefromParent (Variables|Pages|Getnetsettingsui)))

(event Custom|Init%20Net%20Settings
  (bind _netsettingsui (Variables|Pages|Getnetsettingsui))
  (bind _netsettingsui_2 (Variables|Pages|Getnetsettingsui))
  ;[1 1 1] Load Net Settings From Algorand Manager
  (bind _returnvalue (Class|AlgorandUnrealManager|GetAlgodRpcInfo (Variables|Default|GetAlgorandManager)))
  (Utilities|FlowControl|Sequence
    (:then_0
      (Rendering|Components|TextRender|SetText (Variables|/Game/AlgorandUnreal/Blueprint/Widgets/Components/Modals/WBP_MODAL_Net_Setting.WBP_MODAL_Net_Setting_C|GetEditableText_Algod_RPC _netsettingsui_2) (Utilities|Text|ToText(String) (.url (Utilities|Struct|BreakRPCInfo _returnvalue))))
      (bind _returnvalue_2 (Class|AlgorandUnrealManager|GetIndexerRpcInfo (Variables|Default|GetAlgorandManager)))
      (Utilities|FlowControl|Sequence
        (:then_0
          (Rendering|Components|TextRender|SetText (Variables|/Game/AlgorandUnreal/Blueprint/Widgets/Components/Modals/WBP_MODAL_Net_Setting.WBP_MODAL_Net_Setting_C|GetEditableText_Indexer_RPC _netsettingsui) (Utilities|Text|ToText(String) (.url (Utilities|Struct|BreakRPCInfo _returnvalue_2)))))
        (:then_1
          (Rendering|Components|TextRender|SetText (Variables|/Game/AlgorandUnreal/Blueprint/Widgets/Components/Modals/WBP_MODAL_Net_Setting.WBP_MODAL_Net_Setting_C|GetEditableText_Indexer_Port _netsettingsui) (Utilities|Text|ToText(String) (Class|AlgorandBPFunctionLibrary|ToString(FUInt64) (.port (Utilities|Struct|BreakRPCInfo _returnvalue_2))))))
        (:then_2
          (Rendering|Components|TextRender|SetText (Variables|/Game/AlgorandUnreal/Blueprint/Widgets/Components/Modals/WBP_MODAL_Net_Setting.WBP_MODAL_Net_Setting_C|GetEditableText_Indexer_Token _netsettingsui) (Utilities|Text|ToText(String) (.token (Utilities|Struct|BreakRPCInfo _returnvalue_2)))))))
    (:then_1
      (Rendering|Components|TextRender|SetText (Variables|/Game/AlgorandUnreal/Blueprint/Widgets/Components/Modals/WBP_MODAL_Net_Setting.WBP_MODAL_Net_Setting_C|GetEditableText_Algod_Port _netsettingsui_2) (Utilities|Text|ToText(String) (Class|AlgorandBPFunctionLibrary|ToString(FUInt64) (.port (Utilities|Struct|BreakRPCInfo _returnvalue))))))
    (:then_2
      (Rendering|Components|TextRender|SetText (Variables|/Game/AlgorandUnreal/Blueprint/Widgets/Components/Modals/WBP_MODAL_Net_Setting.WBP_MODAL_Net_Setting_C|GetEditableText_Algod_Token _netsettingsui_2) (Utilities|Text|ToText(String) (.token (Utilities|Struct|BreakRPCInfo _returnvalue)))))))

(event EventBeginPlay
  ;[1 1 1] Create First UI
  (if (Utilities|IsValid (Variables|Pages|Getwalletui))
    _
    (else
      (bind _returnvalue (UserInterface|CreateWidget "/Game/AlgorandUnreal/Blueprint/Widgets/Pages/WBP_UI_Wallet.WBP_UI_Wallet_C"))
      (Variables|Pages|Setwalletui _returnvalue)))
  (UserInterface|Viewport|AddtoViewport (Variables|Pages|Getwalletui) 0)
  (CallFunction|InitializeAlgorandManger))

(fn ConstructionScript)

(fn PrintError
  (params (Error :type Error%20Structure))
  (Development|PrintString (Utilities|Struct|BreakError Error)))

(fn ConvertFUInt64toString
  (params (Value :type U%20Int%2064%20Structure))
  (return (Utilities|Text|FormatText (Utilities|Text|ToText(String) (Class|AlgorandBPFunctionLibrary|ToString(FUInt64) Value)))))

(fn ConvertDecimalFStringtoUInt64
  (params (ValueIn :type String))
  (return (Class|AlgorandBPFunctionLibrary|ToUInt64(FString) ValueIn (Class|KismetSystemLibrary|MakeLiteralBool false))))

(fn ConvertFStringtoUInt64
  (params (ValueIn :type String))
  (return (Class|AlgorandBPFunctionLibrary|ToUInt64(FString) ValueIn (Class|KismetSystemLibrary|MakeLiteralBool true))))

(fn LaunchTXLink
  (params (txLink :type String))
  (Utilities|Platform|LaunchURL (Utilities|String|Append "https://testnet.explorer.perawallet.app/tx/" txLink)))

(fn ConvertFUInt64toPeriodString
  (params (value :type U%20Int%2064%20Structure%20%28by%20ref%29))
  (return (Utilities|Text|FormatText (Utilities|Text|ToText(String) (Class|AlgorandBPFunctionLibrary|ToPeriodString(FUInt64) value (Class|AlgorandBPFunctionLibrary|ToUInt64(FString) (Variables|Default|GetDigitCount) (Class|KismetSystemLibrary|MakeLiteralBool true)))))))